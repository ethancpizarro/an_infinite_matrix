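; BP_Tunnel is an endless-runner tunnel segment with a spinning holed wall, a trigger zone and a health pack.
; Passing the trigger adds score, raises player speed by 1% up to a cap, requests the next tunnel from TunnelSpawner and destroys this one.
; Wall hits cost score and health, showing restart at zero health, while the pack heals.
; Separate functions randomize wall mesh and roll, and pack position, usually offset off-centre.
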(event OnComponentBeginOverlap(TriggerZone)
  (params (OverlappedComponent :type Primitive%20Component%20Object%20Reference) (OtherActor :type Actor%20Object%20Reference) (OtherComp :type Primitive%20Component%20Object%20Reference) (OtherBodyIndex :type Integer) (bFromSweep :type Boolean) (SweepResult :type Hit%20Result%20Structure%20%28by%20ref%29))
  (bind _asbp_player (Utilities|Casting|CastToBP_Player OtherActor))
  (bind _output_get (Variables|/Game/InfiniteMatrix/Blueprints/BP_Player.BP_Player_C|SetScore _asbp_player (+ (Variables|/Game/InfiniteMatrix/Blueprints/BP_Player.BP_Player_C|GetScore _asbp_player) 1)))
  (Default|UpdateScore (Variables|/Game/InfiniteMatrix/Blueprints/BP_Player.BP_Player_C|GetScoreReference _asbp_player) _output_get)
  (if (<= (+ (Variables|/Game/InfiniteMatrix/Blueprints/BP_Player.BP_Player_C|GetForwardSpeed _asbp_player) (* (Variables|/Game/InfiniteMatrix/Blueprints/BP_Player.BP_Player_C|GetForwardSpeed _asbp_player) 0.01)) 5e+03)
    (Variables|/Game/InfiniteMatrix/Blueprints/BP_Player.BP_Player_C|SetForwardSpeed _asbp_player (+ (Variables|/Game/InfiniteMatrix/Blueprints/BP_Player.BP_Player_C|GetForwardSpeed _asbp_player) (* (Variables|/Game/InfiniteMatrix/Blueprints/BP_Player.BP_Player_C|GetForwardSpeed _asbp_player) 0.01)))
    (else
      (Variables|/Game/InfiniteMatrix/Blueprints/BP_Player.BP_Player_C|SetForwardSpeed _asbp_player 5e+03)))
  (Default|SpawnTunnelatSpawnPoint (Variables|Default|GetTunnelSpawner))
  (Actor|DestroyActor))

(event OnComponentBeginOverlap(WallMesh)
  (params (OverlappedComponent :type Primitive%20Component%20Object%20Reference) (OtherActor :type Actor%20Object%20Reference) (OtherComp :type Primitive%20Component%20Object%20Reference) (OtherBodyIndex :type Integer) (bFromSweep :type Boolean) (SweepResult :type Hit%20Result%20Structure%20%28by%20ref%29))
  (bind _asbp_player (Utilities|Casting|CastToBP_Player OtherActor))
  (Variables|/Game/InfiniteMatrix/Blueprints/BP_Player.BP_Player_C|SetScore _asbp_player (- (Variables|/Game/InfiniteMatrix/Blueprints/BP_Player.BP_Player_C|GetScore _asbp_player) 1))
  (bind _output_get (Variables|/Game/InfiniteMatrix/Blueprints/BP_Player.BP_Player_C|SetHealth _asbp_player (- (Variables|/Game/InfiniteMatrix/Blueprints/BP_Player.BP_Player_C|GetHealth _asbp_player) 2e+01)))
  (Default|UpdateHealthBar (Variables|/Game/InfiniteMatrix/Blueprints/BP_Player.BP_Player_C|GetHealthBarReference _asbp_player) _output_get)
  (if (<= (Variables|/Game/InfiniteMatrix/Blueprints/BP_Player.BP_Player_C|GetHealth _asbp_player) 0.0)
    (Variables|/Game/InfiniteMatrix/Blueprints/BP_Player.BP_Player_C|SetIsDead _asbp_player true)
    (Default|DisplayRestart _asbp_player)))

(event OnComponentBeginOverlap(HealthPack)
  (params (OverlappedComponent :type Primitive%20Component%20Object%20Reference) (OtherActor :type Actor%20Object%20Reference) (OtherComp :type Primitive%20Component%20Object%20Reference) (OtherBodyIndex :type Integer) (bFromSweep :type Boolean) (SweepResult :type Hit%20Result%20Structure%20%28by%20ref%29))
  (bind _asbp_player (Utilities|Casting|CastToBP_Player OtherActor))
  (if (<= (Variables|/Game/InfiniteMatrix/Blueprints/BP_Player.BP_Player_C|GetHealth _asbp_player) 8e+01)
    (bind _output_get (Variables|/Game/InfiniteMatrix/Blueprints/BP_Player.BP_Player_C|SetHealth _asbp_player (+ (Variables|/Game/InfiniteMatrix/Blueprints/BP_Player.BP_Player_C|GetHealth _asbp_player) 2e+01)))
    (Default|UpdateHealthBar (Variables|/Game/InfiniteMatrix/Blueprints/BP_Player.BP_Player_C|GetHealthBarReference _asbp_player) _output_get)
    (else
      (bind _output_get_2 (Variables|/Game/InfiniteMatrix/Blueprints/BP_Player.BP_Player_C|SetHealth _asbp_player 1e+02))
      (Default|UpdateHealthBar (Variables|/Game/InfiniteMatrix/Blueprints/BP_Player.BP_Player_C|GetHealthBarReference _asbp_player) _output_get_2))))

(event EventBeginPlay)

(event EventTick
  (params (DeltaSeconds :type Float%20%28single-precision%29))
  (Transformation|AddLocalRotation (Variables|Default|GetWallMesh) (Math|Rotator|MakeRotator (* DeltaSeconds (Variables|Default|GetRotateSpeed)) 0.0 0.0) false false))

(fn ConstructionScript)

(fn RandomizeWall
  (Components|StaticMesh|SetStaticMesh (Variables|Default|GetWallMesh) (Utilities|Select :Index (Math|Random|RandomIntegerinRange 0 3) :Option%200 "/Game/InfiniteMatrix/Meshes/SM_Hole_01.SM_Hole_01" :Option%201 "/Game/InfiniteMatrix/Meshes/SM_Hole_02.SM_Hole_02" :Option%202 "/Game/InfiniteMatrix/Meshes/SM_Hole_03.SM_Hole_03" :Option%203 "/Game/InfiniteMatrix/Meshes/SM_Hole_04.SM_Hole_04"))
  (Transformation|AddLocalRotation (Variables|Default|GetWallMesh) (Math|Rotator|MakeRotator (Math|Random|RandomFloatinRange 0.0 3.6e+02) 0.0 0.0) false false))

(fn RandomizeHealth
  (bind _returnvalue (Math|Random|RandomIntegerinRange 0 4))
  (bind _returnvalue_2 (Math|Random|RandomFloatinRange -3e+02 3e+02))
  (bind _returnvalue_3 (Utilities|Select :Index _returnvalue :Option%200 1e+03 :Option%201 1e+03 :Option%202 1e+03 :Option%203 1e+03 :Option%204 _returnvalue_2))
  (Transformation|SetWorldLocation (Variables|Default|GetHealthPack) (Math|Vector|MakeVector (+ (.x (Transformation|GetActorLocation (Game|Player|GetPlayerPawn 0))) (Math|Random|RandomFloatinRange 1e+03 1.5e+03)) _returnvalue_3 _returnvalue_3) false false))